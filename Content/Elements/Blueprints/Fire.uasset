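; Fire projectile actor that damages Damagable actors it overlaps, ignoring those tagged Friendly.
; On BeginPlay it rotates its velocity to the actor's facing, and a timeline shrinks it before toggling off the particle effect and waiting briefly.
; Hitting a non-friendly Damagable spawns a fireball explosion, sends damage through an interface message and destroys the projectile.
; Overlapping anything non-damagable destroys it without an explosion.
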(event `self.Collision.OnComponentBeginOverlap`
  (params (OverlappedComponent :type "PrimitiveComponent Object Reference") (OtherActor :type "Actor Object Reference") (OtherComp :type "PrimitiveComponent Object Reference") (OtherBodyIndex :type Integer) (bFromSweep :type Boolean) (SweepResult :type "HitResult Structure (by ref)"))
  (set `self.DamagedCharacter` OtherActor)
  (if (`KismetSystemLibrary.DoesImplementInterface` OtherActor "/Game/ProjectLibrary/Interfaces/iDamagable.iDamagable_C")
    (if (not (`self.ActorHasTag` OtherActor "Friendly"))
      (`GameplayStatics.SpawnEmitterAtLocation` "/Game/Elements/Fire/P_Explosion_Fireball.P_Explosion_Fireball" (`self.K2_GetActorLocation`)) ; Spawn an impact effect
      (message `/Game/ProjectLibrary/Interfaces/iDamagable.AffectHealth` (`self.DamagedCharacter`) (`self.ArrowDamage`))
      (`self.K2_DestroyActor`))
    (else
      (`self.K2_DestroyActor`))))

(event `self.ReceiveBeginPlay`
  (set `MovementComponent.Velocity` (`KismetMathLibrary.GreaterGreater_VectorRotator` (`self.Velocity`) (`self.K2_GetActorRotation`)) (`self.ProjectileMovement1`)) ; Set the speed/direction of the projectile
  (bind (_direction _scale) (`Timeline|LifeSpan`) ; Timeline blends from 1 to 0.15
    (:`Update`
      (`self.SetActorRelativeScale3D` (* (`KismetMathLibrary.MakeVector` 1.0 1.0 1.0) _scale)) ; Gradually shrink the actor
    )
    (:`Finished`
      (`ActorComponent.ToggleActive` (`self.Effect`)) ; Turn off effect to give particles a chance to fade instead of disappearing suddenly when the actor is destroyed
      (`KismetSystemLibrary.Delay` 0.1))))

(fn `UserConstructionScript`)