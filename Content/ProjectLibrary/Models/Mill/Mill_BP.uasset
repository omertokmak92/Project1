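; Mill actor Blueprint that continuously spins its Cube component, as a turning mill.
; BeginPlay caches the Cube's world roll and yaw, then starts a looping 0.01-second timer bound to DegirmenDonme.
; Each timer call adds a fixed increment to an angle, wraps it at 360 and applies it as world pitch, keeping the cached roll and yaw.
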(event `self.ReceiveBeginPlay`
  (bind (_returnvalue_roll _returnvalue_pitch _returnvalue_yaw) (`KismetMathLibrary.BreakRotator` (`SceneComponent.K2_GetComponentRotation` (`self.Cube`))))
  (set `self.X` _returnvalue_roll)
  (set `self.Z` _returnvalue_yaw)
  (`KismetSystemLibrary.K2_SetTimerDelegate` (delegate `DegirmenDonme`) 0.01 true))

(event `self.ReceiveTick`
  (params (DeltaSeconds :type "Float (single-precision)")))

(event `DegirmenDonme`
  (bind _output_get (set `self.Y` (+ (`self.Y`) 0.5)))
  (`SceneComponent.K2_SetWorldRotation` (`self.Cube`) (`KismetMathLibrary.MakeRotator` (`self.X`) (mod _output_get 360.0) (`self.Z`)) false false))

(fn `UserConstructionScript`)