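; Weapon Blueprint that fires projectiles automatically while its trigger is held.
; PullTrigger passes through a DoOnce, fires immediately and starts a looping timer on Fire at an interval derived from RoundsPerSecond.
; ReleaseTrigger clears that timer and resets the DoOnce for the next pull.
; Each Fire spawns the Projectile class at the ProjectileSpawnPoint transform, regardless of collisions.
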(event `PullTrigger`
  (`/Engine/EditorBlueprintResources/StandardMacros.DoOnce` false :!label _label
    (:`Completed`
      (`self.Fire`)
      (bind _returnvalue (`KismetSystemLibrary.K2_SetTimer` null "Fire" (/ 1.0 (`self.RoundsPerSecond`)) true))
      (set `self.Timer` _returnvalue))))

(event `ReleaseTrigger`
  (`KismetSystemLibrary.K2_ClearAndInvalidateTimerHandle` (`self.Timer`))
  (goto _label :!via `Reset`))

(event `Fire`
  (`|SpawnActorFromClass` "/Game/ProjectLibrary/Blueprints/Projectile/Projectile.Projectile_C" (`SceneComponent.K2_GetComponentToWorld` (`self.ProjectileSpawnPoint`)) "AlwaysSpawn" "OverrideRootScale" null null))

(fn `UserConstructionScript`)