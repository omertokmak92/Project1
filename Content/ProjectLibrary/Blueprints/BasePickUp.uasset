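; Base pickup actor that the third-person character collects into the HUD inventory and can use to restore health, mood and energy.
; The construction script sets the mesh and fills an item info struct from custom fields.
; A trigger shows a prompt widget and arms the pickup event bound to the character, which hides the actor and refreshes the inventory.
; Using it adds to the stats, capped at 1.0, then destroys the actor.
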(event `self.ReceiveBeginPlay`
  (bind _pickuptextreference (`self.PickUpTextReference`))
  (bind (_iteminfo_item _iteminfo_itemimage _iteminfo_pickuptext) (break `/Game/ProjectLibrary/Blueprints/InventoryStruct` (`self.ItemInfo`)))
  ;[1 1 1] Event Begin Play
  (bind _returnvalue (`|CreateWidget` "/Game/ProjectLibrary/UMG/PickUpText.PickUpText_C"))
  (set `self.PickUpTextReference` _returnvalue)
  (setmembers `/Game/ProjectLibrary/Blueprints/InventoryStruct` :`StructRef` (`self.ItemInfo`) :`Item` self)
  (set `/Game/ProjectLibrary/UMG/PickUpText.PickUpActor` _iteminfo_item _pickuptextreference)
  (set `/Game/ProjectLibrary/UMG/PickUpText.PickUpText` _iteminfo_pickuptext _pickuptextreference)
  (bind _asthird_person_character (cast `/Game/ThirdPersonBP/Blueprints/ThirdPersonCharacter` (`GameplayStatics.GetPlayerCharacter` 0)))
  (bind _output_get (set `self.CharacterReference` _asthird_person_character))
  (add `/Game/ThirdPersonBP/Blueprints/ThirdPersonCharacter.PickUpItem` _output_get (delegate `PickUpItem_Event`)))

(event `self.Trigger.OnComponentBeginOverlap`
  (params (OverlappedComponent :type "PrimitiveComponent Object Reference") (OtherActor :type "Actor Object Reference") (OtherComp :type "PrimitiveComponent Object Reference") (OtherBodyIndex :type Integer) (bFromSweep :type Boolean) (SweepResult :type "HitResult Structure (by ref)"))
  ;[1 1 1] Overlap Trigger Script
  (cast `/Game/ThirdPersonBP/Blueprints/ThirdPersonCharacter` OtherActor)
  (`UserWidget.AddToViewport` (`self.PickUpTextReference`) 0)
  (set `self.IsInRange` true))

(event `PickUpItem_Event`
  ;[1 1 1] Pick up and add item to inventory then refresh it
  (if (and (`self.IsInRange`) (`self.GetActorEnableCollision`))
    (`KismetArrayLibrary.Array_Add` (`/Game/ProjectLibrary/UMG/GameHud.Inventory` (`/Game/ThirdPersonBP/Blueprints/ThirdPersonCharacter.GameHudReference` (`self.CharacterReference`))) (`self.ItemInfo`))
    (`Widget.RemoveFromParent` (`self.PickUpTextReference`))
    (`self.SetActorHiddenInGame` true)
    (`self.SetActorEnableCollision` false)
    (`/Game/ProjectLibrary/UMG/GameHud.RefreshInventory` (`/Game/ThirdPersonBP/Blueprints/ThirdPersonCharacter.GameHudReference` (`self.CharacterReference`)))))

(event `self.Trigger.OnComponentEndOverlap`
  (params (OverlappedComponent :type "PrimitiveComponent Object Reference") (OtherActor :type "Actor Object Reference") (OtherComp :type "PrimitiveComponent Object Reference") (OtherBodyIndex :type Integer))
  ;[1 1 1] Overlap Trigger Script
  (cast `/Game/ThirdPersonBP/Blueprints/ThirdPersonCharacter` OtherActor)
  (`Widget.RemoveFromParent` (`self.PickUpTextReference`))
  (set `self.IsInRange` false))

(event `/Game/ProjectLibrary/Blueprints/ActionInterface.UseAction`
  ;[1 1 1] Use Action
  (`self.Add Health`)
  (`self.Add Mood`)
  (`self.Add Energy`)
  (`self.K2_DestroyActor`))

(event `Add Health`
  (bind _characterreference (`self.CharacterReference`))
  (bind _returnvalue (+ (`/Game/ThirdPersonBP/Blueprints/ThirdPersonCharacter.HealthValue` (`self.CharacterReference`)) (`self.AddHealth`)))
  ;[1 1 1] Add Health Function
  (if (< _returnvalue 1.0)
    (set `/Game/ThirdPersonBP/Blueprints/ThirdPersonCharacter.HealthValue` _returnvalue _characterreference)
    (else
      (set `/Game/ThirdPersonBP/Blueprints/ThirdPersonCharacter.HealthValue` 1.0 _characterreference))))

(event `Add Energy`
  (bind _characterreference (`self.CharacterReference`))
  (bind _returnvalue (+ (`/Game/ThirdPersonBP/Blueprints/ThirdPersonCharacter.EnergyValue` (`self.CharacterReference`)) (`self.AddEnergy`)))
  ;[1 1 1] Add Energy Function
  (if (< _returnvalue 1.0)
    (set `/Game/ThirdPersonBP/Blueprints/ThirdPersonCharacter.EnergyValue` _returnvalue _characterreference)
    (else
      (set `/Game/ThirdPersonBP/Blueprints/ThirdPersonCharacter.EnergyValue` 1.0 _characterreference))))

(event `Add Mood`
  (bind _characterreference (`self.CharacterReference`))
  (bind _returnvalue (+ (`/Game/ThirdPersonBP/Blueprints/ThirdPersonCharacter.MoodValue` (`self.CharacterReference`)) (`self.AddMood`)))
  ;[1 1 1] Add Mood Function
  (if (< _returnvalue 1.0)
    (set `/Game/ThirdPersonBP/Blueprints/ThirdPersonCharacter.MoodValue` _returnvalue _characterreference)
    (else
      (set `/Game/ThirdPersonBP/Blueprints/ThirdPersonCharacter.MoodValue` 1.0 _characterreference))))

(fn `UserConstructionScript`
  (bind _structout (setmembers `/Game/ProjectLibrary/Blueprints/InventoryStruct` :`StructRef` (make `/Game/ProjectLibrary/Blueprints/InventoryStruct` self (`self.CustomImage`) (`self.CustomPickUpText`) (`self.CustomActionText`))))
  (set `self.ItemInfo` _structout)
  (`StaticMeshComponent.SetStaticMesh` (`self.StaticMesh`) (`self.CustomStaticMesh`)))