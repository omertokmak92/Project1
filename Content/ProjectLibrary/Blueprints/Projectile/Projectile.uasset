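; Projectile actor that deals bullet damage to damageable targets it touches.
; On sphere overlap, it checks the other actor for the IDamagable interface and skips those tagged Friendly.
; Non-friendly damageable actors receive BulletDamage through AffectHealthMessage, and the projectile destroys itself on them or on any non-damageable actor, passing through friendlies.
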(event `self.Sphere.OnComponentBeginOverlap`
  (params (OverlappedComponent :type "PrimitiveComponent Object Reference") (OtherActor :type "Actor Object Reference") (OtherComp :type "PrimitiveComponent Object Reference") (OtherBodyIndex :type Integer) (bFromSweep :type Boolean) (SweepResult :type "HitResult Structure (by ref)"))
  (set `self.DamagedCharacter` OtherActor)
  (if (`KismetSystemLibrary.DoesImplementInterface` OtherActor "/Game/ProjectLibrary/Interfaces/iDamagable.iDamagable_C")
    (if (not (`self.ActorHasTag` OtherActor "Friendly"))
      (message `/Game/ProjectLibrary/Interfaces/iDamagable.AffectHealth` (`self.DamagedCharacter`) (`self.BulletDamage`))
      (`self.K2_DestroyActor`))
    (else
      (`self.K2_DestroyActor`))))

(fn `UserConstructionScript`)